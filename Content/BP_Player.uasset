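; Physics-driven player pawn with movement along world Y, limited multi-jump and a dash.
; Jumps are velocity-change impulses that weaken per jump, gated by a delay after button release and reset on Tick when not falling.
; Dash cancels current velocity, drives Y velocity from a timeline, and lowers drag, which a looping timer restores.
; Alternative timer-based dash and double-tap logic remain as unwired leftovers.
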(event `Reset Dash`
  ;[0.8181 0.6561 1] Alternative Dashing Nodes
  (`/Engine/EditorBlueprintResources/StandardMacros.DoOnce` false :!via `Reset`
    (:`Completed`
      (set `self.Stored time` (`GameplayStatics.GetTimeSeconds`))
      (set `self.Count` 0))))

(event `InputAction|Dash`
  (params (Key :type "Key Structure"))
  ;[0.8181 0.6561 1] Alternative Dashing Nodes
)

(event `applyVel`
  ;[0.8181 0.6561 1] Alternative Dashing Nodes
  (`/Engine/EditorBlueprintResources/StandardMacros.IncrementInt` (`self.Count`)
    (:`  `
      (set `self.Dashing` true)
      (`PrimitiveComponent.SetAllPhysicsLinearVelocity` (`self.Box`) (`KismetMathLibrary.MakeVector` 0.0 (* (`self.AltDashVelocity`) 5000.0)) false)
      (if (>= (`self.Count`) 30)
        (`KismetSystemLibrary.K2_ClearTimer` null "applyVel")
        (`self.Reset Dash`)))))

(event `InputAction|Dash`
  (params (Key :type "Key Structure"))
  (:`Pressed`
    (`self.Dash Function` -1.0)
    (bind (_direction _y_track) (`Timeline|Dash Timeline` :!via `PlayFromStart`)
      (:`Update`
        (`PrimitiveComponent.SetAllPhysicsLinearVelocity` (`self.Box`) (`KismetMathLibrary.MakeVector` 0.0 _y_track) false)
        (set `/Game/BP_MoveComponent.DragMultiplier` 0.3 (`self.BP_MoveComponent`))
        (`self.Momentum Decay`)))))

(event `Momentum Decay`
  (`KismetSystemLibrary.K2_SetTimerDelegate` (delegate `DragReset`) 0.25 true))

(event `DragReset`
  (bind _bp_movecomponent (`self.BP_MoveComponent`))
  (bind _output_get (set `/Game/BP_MoveComponent.DragMultiplier` (`KismetMathLibrary.FClamp` (+ (`/Game/BP_MoveComponent.DragMultiplier` _bp_movecomponent) 0.05) 0.0 0.9) _bp_movecomponent))
  (if (>= _output_get 0.9)
    (`KismetSystemLibrary.K2_ClearTimer` null "DragReset")))

(event `InputAxis|Move Right`
  (params (AxisValue :type "Float (single-precision)"))
  (if (`self.Movement Input Check`)
    (`self.AddMovementInput` (`KismetMathLibrary.MakeVector` 0.0 AxisValue))))

(event `InputAction|Jump`
  (params (Key :type "Key Structure"))
  (:`Pressed`
    (bind _counter (`/Engine/EditorBlueprintResources/StandardMacros.Do N` (`self.Max Jumps`) :!label _label)
      (:`Exit`
        (`/Engine/EditorBlueprintResources/StandardMacros.Gate` false :!label _label_2
          (:`Exit`
            (`self.Jump Function` (`KismetMathLibrary.FClamp` (/ (`self.Jump Decay Modifier`) (`KismetMathLibrary.Conv_IntToDouble` _counter)) (`self.Minimum Jump Power`) 5.0) (`self.Jump Strength`))
            (`self.Close Jump Gate`))))))
  (:`Released`
    (`KismetSystemLibrary.Delay` (`self.DoubleJumpDelay`))
    (`self.Open Jump Gate`)))

(event `Open Jump Gate`
  (goto _label_2 :!via `Open`))

(event `Close Jump Gate`
  (goto _label_2 :!via `Close`))

(event `self.ReceiveTick`
  (params (DeltaSeconds :type "Float (single-precision)"))
  (if (not (`/Game/BP_MoveComponent.Pawn Is Falling` (`self.BP_MoveComponent`)))
    (goto _label :!via `Reset`)))

(fn `Dash Function`
  (params (`Direction Multiplier` :type "Float (double-precision)"))
  (locals (VelocityBeforeDash :type "Float (double-precision)"))
  (bind _bp_movecomponent (`self.BP_MoveComponent`))
  (bind (_returnvalue_x _returnvalue_y _returnvalue_z) (`KismetMathLibrary.BreakVector` (* (`/Game/BP_MoveComponent.Velocity` _bp_movecomponent) -1.0)))
  (`/Game/BP_MoveComponent.Deconfigure Physics` _bp_movecomponent)
  (set `self.Movement Input Check` false)
  (`PrimitiveComponent.AddImpulse` (`self.Box`) (`KismetMathLibrary.MakeVector` _returnvalue_x _returnvalue_y _returnvalue_z) "None" true)
  (`/Game/BP_MoveComponent.Configure Physics` (`self.BP_MoveComponent`))
  (set `self.Movement Input Check` true))

(fn `Jump Function`
  (params (`Jump Strength Modifier` :type "Float (double-precision)") (`Jump Strength` :type "Float (double-precision)"))
  (bind (_velocity_x _velocity_y _velocity_z) (`KismetMathLibrary.BreakVector` (`/Game/BP_MoveComponent.Velocity` (`self.BP_MoveComponent`))))
  (`PrimitiveComponent.AddImpulse` (`self.Box`) (`KismetMathLibrary.MakeVector` 0.0 (/ _velocity_y (`self.Y Impulse on Jump`)) (+ (* (* `Jump Strength Modifier` _velocity_z) -1.0) `Jump Strength`)) "None" true))

(fn `UserConstructionScript`)
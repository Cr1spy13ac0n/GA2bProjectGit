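; RisingPlatform is an actor that repeatedly shakes, launches upward, then sinks back to its start.
; The RiseAndFall timeline jitters the actor in X and Y around the platform's original location, then its Launch event starts the Launch timeline.
; That timeline raises Plat until it passes Height, then sets Falling.
; Tick lowers Plat slowly and restarts the cycle at the bottom, using fixed per-frame steps without delta-time scaling.
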(event `self.ReceiveBeginPlay`
  (bind _plat (`self.plat`))
  (bind (_originallocation_x _originallocation_y _originallocation_z) (`KismetMathLibrary.BreakVector` (`self.OriginalLocation`)))
  (bind (_returnvalue_x _returnvalue_y _returnvalue_z) (`KismetMathLibrary.BreakVector` (`SceneComponent.K2_GetComponentLocation` _plat)))
  (set `self.OriginalLocation` (`SceneComponent.K2_GetComponentLocation` (`self.plat`)))
  (`Timeline|Rise and Fall` :!via `PlayFromStart` :!label _label
    (:`Update`
      (`self.Shake`))
    (:`Launch`
      (`Timeline|Launch` :!via `PlayFromStart` :!label _label_2
        (:`Update`
          (if (< _returnvalue_z (+ _originallocation_z (`self.Height`)))
            (`SceneComponent.K2_AddWorldOffset` _plat (0.0 0.0 15.0) false false)
            (else
              (set `self.Falling` true)
              (goto _label_2 :!via `Stop`))))))))

(event `self.ReceiveTick`
  (params (DeltaSeconds :type "Float (single-precision)"))
  (bind (_originallocation_x _originallocation_y _originallocation_z) (`KismetMathLibrary.BreakVector` (`self.OriginalLocation`)))
  (bind (_returnvalue_x _returnvalue_y _returnvalue_z) (`KismetMathLibrary.BreakVector` (`SceneComponent.K2_GetComponentLocation` (`self.plat`))))
  (if (`self.Falling`)
    (if (< _returnvalue_z _originallocation_z)
      (set `self.Falling` false)
      (goto _label :!via `PlayFromStart`)
      (else
        (`SceneComponent.K2_AddWorldOffset` (`self.plat`) (0.0 0.0 -2.0) false false)))))

(fn `Shake`
  (bind _output_get (set `self.Offset` (`KismetMathLibrary.MakeVector` (`KismetMathLibrary.RandomFloatInRange` -2.0 2.0) (`KismetMathLibrary.RandomFloatInRange` -2.0 2.0))))
  (`self.K2_SetActorLocation` (+ _output_get (`self.OriginalLocation`))))

(fn `UserConstructionScript`)
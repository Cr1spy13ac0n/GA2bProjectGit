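; Default player controller that opens the pause menu when the Pause input is pressed.
; PauseGame creates a new WBP_PauseMenu, stores it, adds it to the viewport, pauses the game and shows the mouse cursor.
; Unpause logic that would remove the menu and hide the cursor is present but disconnected, and the Ting flag is set but never read.
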(event `InputAction|Pause`
  (params (Key :type "Key Structure"))
  (:`Pressed`
    (`self.PauseGame`)))

(fn `PauseGame`
  (bind _returnvalue (`|CreateWidget` "/Game/Blueprints/WBP_PauseMenu.WBP_PauseMenu_C" (`GameplayStatics.GetPlayerController` 0)))
  (bind _output_get (set `self.Pause Menu` _returnvalue))
  (`UserWidget.AddToViewport` _output_get 0)
  (`GameplayStatics.SetGamePaused` true)
  (set `self.bShowMouseCursor` true)
  (set `self.ting` true))

(fn `UserConstructionScript`)
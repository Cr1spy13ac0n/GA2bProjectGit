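; Movement component that drives a Pawn through its physics-simulated box root, held upright and locked to the X=0 plane.
; Tick consumes movement input, resets rotation and X, and line-traces below the box to set the falling state.
; A looping fixed-step timer clamps velocity, adds separate rise and fall gravity atop engine gravity, applies air control, acceleration and drag, then writes the velocity to the body.
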(event `self.ReceiveBeginPlay`
  (bind _aspawn (cast `Pawn` (`self.GetOwner`)))
  (bind _output_get (set `self.Parent` _aspawn))
  (bind _asbox_collision (cast `BoxComponent` (`Actor.RootComponent` _output_get)))
  (set `self.Box Collision` _asbox_collision)
  (`self.Configure Physics`)
  (bind _output_get_2 (set `self.ManualDeltaTime` (`self.ManualDeltaTime`)))
  (`KismetSystemLibrary.K2_SetTimerDelegate` (delegate `Fixed Tick`) _output_get_2 true))

(event `Fixed Tick`
  (bind _output_get (set `self.Velocity` (`SceneComponent.GetComponentVelocity` (`self.Box Collision`))))
  (set `self.Velocity` (`KismetMathLibrary.ClampVectorSize` _output_get 0.0 (`self.Max Velocity`)))
  (`self.Apply Gravity` (`self.Custom Gravity Enabled`))
  (`self.Air Physics`)
  (`self.Movement Velocity` (`self.Strafe Speed`) (`self.Acceleration`) 20.0)
  (`PrimitiveComponent.SetAllPhysicsLinearVelocity` (`self.Box Collision`) (`self.Velocity`) false))

(event `self.ReceiveTick`
  (params (DeltaSeconds :type "Float (single-precision)"))
  (bind (_returnvalue_x _returnvalue_y _returnvalue_z) (`KismetMathLibrary.BreakVector` (`SceneComponent.K2_GetComponentLocation` (`self.Box Collision`))))
  (`self.Is Falling`)
  (bind _parent (`self.Parent`)
    (:`then`
      (bind _returnvalue (`Pawn.ConsumeMovementInputVector` _parent))
      (set `self.Input` (`KismetMathLibrary.Normal` _returnvalue))
      (`SceneComponent.K2_SetWorldRotation` :`self` (`self.Box Collision`))
      (`SceneComponent.K2_SetWorldLocation` (`self.Box Collision`) (`KismetMathLibrary.MakeVector` 0.0 _returnvalue_y _returnvalue_z) false false))
    (:`else`)))

(fn `Air Physics`
  (if (`self.Pawn Is Falling`)
    (set `self.Input` (* (`self.Input`) (`self.Air Control`)))))

(fn `Apply Gravity`
  (params (`Gravity Enabled` :type Boolean))
  (locals (NewLocalVar_0 :type "Vector Structure" :default (0.0 0.0 0.0)))
  (bind (_velocity_x _velocity_y _velocity_z) (`KismetMathLibrary.BreakVector` (`self.Velocity`)))
  (if `Gravity Enabled`
    (if (<= _velocity_z 0.0)
      ;[1 1 1 1 15] Negative constant gravity multiplier being added to current velocity every 'Delta Time'
      (set `self.Velocity` (+ (`self.Velocity`) (* (* (`self.Gravity Direction`) (`self.Down Gravity Scalar`)) (`self.ManualDeltaTime`))))
      (else
        (set `self.Velocity` (+ (`self.Velocity`) (* (* (`self.Gravity Direction`) (`self.Gravity Scalar`)) (`self.ManualDeltaTime`))))))))

(fn `Configure Physics`
  (`self.SetTickGroup` "TG_PostPhysics")
  (`PrimitiveComponent.SetSimulatePhysics` (`self.Box Collision`) true)
  (`PrimitiveComponent.SetEnableGravity` (`self.Box Collision`) true)
  (`PrimitiveComponent.SetCollisionProfileName` (`self.Box Collision`) "BlockAll" true)
  (`PrimitiveComponent.SetPhysMaterialOverride` (`self.Box Collision`) "/Game/Blueprints/M_PawnPhysMaterial.M_PawnPhysMaterial")
  (set `self.Custom Gravity Enabled` true))

(fn `Deconfigure Physics`
  (`PrimitiveComponent.SetEnableGravity` (`self.Box Collision`) false)
  (set `self.Custom Gravity Enabled` false))

(fn `Is Falling`
  (bind (_returnvalue_x _returnvalue_y _returnvalue_z) (`KismetMathLibrary.BreakVector` (`SceneComponent.K2_GetComponentLocation` (`self.Box Collision`))))
  (bind (_returnvalue_x_2 _returnvalue_y_2 _returnvalue_z_2) (`KismetMathLibrary.BreakVector` (`SceneComponent.K2_GetComponentLocation` (`self.Box Collision`))))
  (bind (_outhit _returnvalue) (`KismetSystemLibrary.LineTraceSingle` :`Start` (`KismetMathLibrary.MakeVector` _returnvalue_x_2 _returnvalue_y_2 (- _returnvalue_z_2 30.0)) :`End` (- (`KismetMathLibrary.MakeVector` _returnvalue_x _returnvalue_y (- _returnvalue_z 30.0)) (0.0 0.0 10.0)) :`TraceChannel` "TraceTypeQuery1" :`DrawDebugType` "Persistent"))
  (if _returnvalue
    (if (and _returnvalue (`self.Pawn Is Falling`))
      (set `self.Pawn Is Falling` false)
      (`KismetSystemLibrary.PrintString` "not falling"))
    (elif (`KismetMathLibrary.BooleanNAND` _returnvalue (`self.Pawn Is Falling`))
      (set `self.Pawn Is Falling` true)
      (`KismetSystemLibrary.PrintString` "falling"))))

(fn `Movement Velocity`
  (params (`Strafe Speed` :type "Float (double-precision)") (Acceleration :type "Float (double-precision)") (Deceleration :type "Float (double-precision)"))
  ;[0.5869 0.6123 1] Acceleration
  (set `self.Velocity` (+ (* (- (* (* (`self.Input`) `Strafe Speed`) Acceleration) (`self.Deceleration/Drag` Deceleration)) (`self.ManualDeltaTime`)) (`self.Velocity`))))
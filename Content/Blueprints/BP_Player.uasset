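; Player pawn for a 2D side-scrolling platformer, with physics-driven movement, multi-jump and dash sharing an energy limit that updates the HUD.
; Dash runs on a looping timer, ramping velocity through DashMaths intervals until a box trace hits or the count ends, then drag rises to fake momentum.
; A per-tick ground trace handles landing and energy refill, alongside flipbook swaps and timeline squash-and-stretch.
; Overlapping BP_EndZone shows the end screen.
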(event `InputAction|Dash`
  (params (Key :type "Key Structure")))

(event `self.ReceiveBeginPlay`
  ;[1 0.2525 0] squish n strech
  (set `self.Base scale` (`SceneComponent.RelativeScale3D` (`self.SpriteFB`))))

(event `jump squeeze`
  ;[1 0.2525 0] squish n strech
)

(event `landsquash`
  ;[1 0.2525 0] squish n strech
  (bind (_direction _alpha) (`Timeline|landsquash anim` :!via `PlayFromStart`)
    (:`Update`
      (`SceneComponent.SetRelativeScale3D` (`self.SpriteFB`) (`KismetMathLibrary.VLerp` (`self.Base scale`) (* (`self.Base scale`) (`self.land squash factor`)) _alpha)))))

(event `Test`
  (`PaperFlipbookComponent.SetFlipbook` (`self.SpriteFB`) "/Game/Assets/2D/2d_character_asset/animations/FP_landing.FP_landing")
  (`KismetSystemLibrary.RetriggerableDelay` 0.2)
  (if (`self.temp`)
    ;[1 0.2525 0] squish n strech
    (`PaperFlipbookComponent.SetFlipbook` (`self.SpriteFB`) "/Game/Assets/2D/2d_character_asset/animations/FP_Idle.FP_Idle")))

(event `dash squeez`
  ;[1 0.2525 0] squish n strech
  (bind (_direction _alpha) (`Timeline|dash stretch` :!via `PlayFromStart`)
    (:`Update`
      (`SceneComponent.SetRelativeScale3D` (`self.SpriteFB`) (`KismetMathLibrary.VLerp` (`self.Base scale`) (* (`self.Base scale`) (`self.dash squeeze`)) _alpha)))))

(event `dash_overshoot`
  ;[1 0.2525 0] squish n strech
  (bind (_direction _alpha) (`Timeline|dashovershootanim` :!via `PlayFromStart`)
    (:`Update`
      (`SceneComponent.SetRelativeScale3D` (`self.SpriteFB`) (`KismetMathLibrary.VLerp` (`self.Base scale`) (* (`self.Base scale`) (`self.dash overshoot`)) _alpha)))))

(event `Reset Dash`
  ;[0.724 0.01 0.02258] Do Once Prevents Chain Dashing and also Resets the Counter
  (goto _label_2 :!via `Reset`))

(event `InputAction|Dash`
  (params (Key :type "Key Structure"))
  (:`Pressed`
    (if (`self.Energy Depleted`)
      ;[1 0.3162 0] Energy Depleted Anim
      (`PaperFlipbookComponent.SetFlipbook` (`self.SpriteFB`) "/Game/Assets/2D/2d_character_asset/animations/FP_enegrydepleted.FP_enegrydepleted")
      (`KismetSystemLibrary.Delay` 0.2)
      (`PaperFlipbookComponent.SetFlipbook` (`self.SpriteFB`) "/Game/Assets/2D/2d_character_asset/animations/FP_Idle.FP_Idle")
      (else
        (`|ExecutionSequence`
          (:`then_0`
            (`self.dash squeez`)
            ;[1 0.2368 0] Sets Anim To Appropriate State
            (`PaperFlipbookComponent.SetFlipbook` (`self.SpriteFB`) "/Game/Assets/2D/2d_character_asset/animations/FP_Dash.FP_Dash")
            (bind _energy_remaining (`self.Energy System`))
            (`KismetSystemLibrary.PrintString` (`KismetStringLibrary.Conv_IntToString` _energy_remaining))
            (`/Game/Blueprints/BP_MoveComponent.Deconfigure Physics` (`self.BP_MoveComponent`))
            (set `self.Movement Input Check` false)
            ;[0.724 0.01 0.02258] Determines Dash Direction
            (if (`self.MovingRight`)
              (set `self.Direction Determiner` 1)
              (`|ExecutionSequence` :!label _label
                (:`then_0`
                  ;[0.724 0.01 0.02258] Do Once Prevents Chain Dashing and also Resets the Counter
                  (`/Engine/EditorBlueprintResources/StandardMacros.DoOnce` false :!label _label_2
                    (:`Completed`
                      (set `self.Count` 0))))
                (:`then_1`
                  (`KismetSystemLibrary.K2_SetTimerDelegate` (delegate `ApplyVel`) (/ (`self.Dash Time`) (`self.Max Counter`)) true)))
              (elif (not (`self.MovingRight`))
                (set `self.Direction Determiner` -1)
                (goto _label))))
          (:`then_1`
            (if (`/Game/Blueprints/BP_MoveComponent.Pawn Is Falling` (`self.BP_MoveComponent`))
              (`PaperFlipbookComponent.SetFlipbook` (`self.SpriteFB`) "/Game/Assets/2D/2d_character_asset/animations/FP_air.FP_air"))))))))

(event `ApplyVel`
  (bind (_outgoingmaximumvel _returnvalue _outgoingmaximumcount) (`self.DashMaths` 0.13 0.0 0.55))
  (bind _box (`self.Box`))
  (bind _box_2 (`self.Box`))
  (bind (_outgoingmaximumvel_2 _returnvalue_2 _outgoingmaximumcount_2) (`self.DashMaths` 0.3 _outgoingmaximumcount 0.8 _outgoingmaximumvel))
  (bind (_returnvalue_x _returnvalue_y _returnvalue_z) (`KismetMathLibrary.BreakVector` (+ (`SceneComponent.K2_GetComponentLocation` _box) (`SceneComponent.GetRightVector` _box))))
  (bind (_returnvalue_x_2 _returnvalue_y_2 _returnvalue_z_2) (`KismetMathLibrary.BreakVector` (+ (`SceneComponent.K2_GetComponentLocation` _box_2) (`SceneComponent.GetRightVector` _box_2))))
  ;[0.724 0.01 0.02258] If Object is Hit Cancel Dash
  (bind (_outhit _returnvalue_3) (`KismetSystemLibrary.BoxTraceSingle` :`Start` (`KismetMathLibrary.MakeVector` _returnvalue_x_2 (- _returnvalue_y_2 30.0) _returnvalue_z_2) :`End` (`KismetMathLibrary.MakeVector` _returnvalue_x (- _returnvalue_y -30.0) _returnvalue_z) :`HalfSize` (10.0 10.0 10.0) :`TraceChannel` "TraceTypeQuery1" :`DrawDebugType` "Persistent"))
  (if _returnvalue_3
    ;[0.724 0.01 0.02258] Resets Dash, Clears the Collision Detection and Re-enables Movement. Checks if the Player is on the Ground to Check if an Energy Reset is Needed
    (`KismetSystemLibrary.K2_ClearTimer` null "ApplyVel")
    (`self.Reset Dash`)
    (`/Game/Blueprints/BP_MoveComponent.Configure Physics` (`self.BP_MoveComponent`))
    (set `self.Movement Input Check` true)
    (if (not (`self.NotLanded`))
      (set `self.EnergyCounter` 0)
      (set `self.Energy Depleted` false))
    (else
      ;[0.724 0.01 0.02258] Counts +1 Every Excecution
      (`/Engine/EditorBlueprintResources/StandardMacros.IncrementInt` (`self.Count`)
        (:`  `
          (set `self.Dashing` true)
          (if (>= (`self.Count`) (`KismetMathLibrary.FTrunc` (* (`self.Max Counter`) 0.55)))
            (if (>= (`self.Count`) (`KismetMathLibrary.FTrunc` (* (`self.Max Counter`) 0.8)))
              ;[0.724 0.01 0.02258] When Count is at 1.0 of the Max Counters Value, Return True.
              (if (>= (`self.Count`) (`KismetMathLibrary.FTrunc` (* (`self.Max Counter`) 1.0)))
                (`KismetSystemLibrary.K2_ClearTimer` null "ApplyVel")
                (`self.Reset Dash`)
                ;[0 0.5625 0.05192] Reduces the Drag Multiplier After Dash To Simulate Momentum
                (set `/Game/Blueprints/BP_MoveComponent.DragMultiplier` 0.3 (`self.BP_MoveComponent`))
                (`self.Momentum Decay`)
                (`/Game/Blueprints/BP_MoveComponent.Configure Physics` (`self.BP_MoveComponent`))
                (set `self.Movement Input Check` true)
                (if (not (`self.NotLanded`))
                  (set `self.EnergyCounter` 0)
                  (set `self.Energy Depleted` false))
                (else
                  (`PrimitiveComponent.SetAllPhysicsLinearVelocity` (`self.Box`) (`KismetMathLibrary.MakeVector` 0.0 (`.ReturnValue` (`self.DashMaths` 1.0 _outgoingmaximumcount_2 1.0 _outgoingmaximumvel_2))) false)))
              (else
                ;[0.724 0.01 0.02258] Repeated Interval, and so on.
                (`PrimitiveComponent.SetAllPhysicsLinearVelocity` (`self.Box`) (`KismetMathLibrary.MakeVector` 0.0 _returnvalue_2) false)))
            (else
              ;[0.724 0.01 0.02258 1 13] Velocity For This Interval. Its Value is Lerped Between the Previous Intervals Max and This Intervals Max.
              (`PrimitiveComponent.SetAllPhysicsLinearVelocity` (`self.Box`) (`KismetMathLibrary.MakeVector` 0.0 _returnvalue) false))))))))

(event `Momentum Decay`
  ;[0 0.5625 0.05192] Increases Drag by x Amount per Excecution to Simulate Artifical Momentum
  (`KismetSystemLibrary.K2_SetTimerDelegate` (delegate `DragReset`) 0.25 true))

(event `DragReset`
  (bind _bp_movecomponent (`self.BP_MoveComponent`))
  ;[0 0.5625 0.05192] Increases Drag by x Amount per Excecution to Simulate Artifical Momentum
  (bind _output_get (set `/Game/Blueprints/BP_MoveComponent.DragMultiplier` (`KismetMathLibrary.FClamp` (+ (`/Game/Blueprints/BP_MoveComponent.DragMultiplier` _bp_movecomponent) 0.05) 0.5 0.9) _bp_movecomponent))
  ;[0 0.5625 0.05192] Once Momentum >= Max Drag Clear Timer
  (if (>= _output_get 0.9)
    (`KismetSystemLibrary.K2_ClearTimer` null "DragReset")))

(event `InputAxis|Move Right`
  (params (AxisValue :type "Float (single-precision)"))
  (bind _papersprite (`self.PaperSprite`))
  (bind _papersprite_2 (`self.PaperSprite`))
  (bind (_relativescale3d_x _relativescale3d_y _relativescale3d_z) (`KismetMathLibrary.BreakVector` (`SceneComponent.RelativeScale3D` _papersprite)))
  (bind (_relativescale3d_x_2 _relativescale3d_y_2 _relativescale3d_z_2) (`KismetMathLibrary.BreakVector` (`SceneComponent.RelativeScale3D` _papersprite_2)))
  (bind _output_get (set `self.Axis Value` AxisValue))
  (if (`self.Movement Input Check`)
    (if (> (`self.Axis Value`) 0.05)
      (set `self.MovingRight` true)
      (`SceneComponent.SetRelativeScale3D` _papersprite (`KismetMathLibrary.MakeVector` 0.11 _relativescale3d_y _relativescale3d_z))
      (`self.AddMovementInput` (`KismetMathLibrary.MakeVector` 0.0 _output_get) :!label _label_3)
      (elif (< (`self.Axis Value`) -0.05)
        (set `self.MovingRight` false)
        (`SceneComponent.SetRelativeScale3D` _papersprite_2 (`KismetMathLibrary.MakeVector` -0.11 _relativescale3d_y_2 _relativescale3d_z_2))
        (goto _label_3)))))

(event `InputAction|Jump`
  (params (Key :type "Key Structure"))
  (:`Pressed`
    (`KismetSystemLibrary.PrintString` (`KismetStringLibrary.Concat_StrStr` "Energy Counter: " (`KismetStringLibrary.Conv_IntToString` (`self.EnergyCounter`))) true true (struct :`R` 0.392701 :`G` 1.0 :`B` 0.388869 :`A` 1.0))
    (if (not (`self.Energy Depleted`))
      ;[1 0.2558 0] jump start animation
      (`self.jump squeeze`)
      (`PaperFlipbookComponent.SetFlipbook` (`self.SpriteFB`) "/Game/Assets/2D/2d_character_asset/animations/FP_Jumpstart.FP_Jumpstart")
      (bind _counter (`/Engine/EditorBlueprintResources/StandardMacros.Do N` (`self.Max Jumps`) :!label _label_4)
        (:`Exit`
          (`/Engine/EditorBlueprintResources/StandardMacros.Gate` false :!label _label_5
            (:`Exit`
              (`self.Jump Function` 0.0 (`self.Jump Strength`))
              (`self.Close Jump Gate`)
              (bind _energy_remaining (`self.Energy System`))
              (`KismetSystemLibrary.PrintString` (`KismetStringLibrary.Conv_IntToString` _energy_remaining))
              (`KismetSystemLibrary.Delay` 0.42)
              (`PaperFlipbookComponent.SetFlipbook` (`self.SpriteFB`) "/Game/Assets/2D/2d_character_asset/animations/FP_air.FP_air")))))))
  (:`Released`
    (`KismetSystemLibrary.Delay` (`self.DoubleJumpDelay`))
    (`self.Open Jump Gate`)))

(event `Open Jump Gate`
  (goto _label_5 :!via `Open`))

(event `Close Jump Gate`
  (goto _label_5 :!via `Close`))

(event `self.ReceiveTick`
  (params (DeltaSeconds :type "Float (single-precision)"))
  (bind _returnvalue (`PrimitiveComponent.GetPhysicsLinearVelocity` (`self.Box`) "None"))
  (`KismetSystemLibrary.PrintString` (`KismetStringLibrary.Conv_VectorToString` _returnvalue) true true (struct :`R` 1.0 :`G` 0.27681 :`B` 0.417032 :`A` 1.0) DeltaSeconds)
  (`self.On Landed`)
  (if (`/Game/Blueprints/BP_MoveComponent.Pawn Is Falling` (`self.BP_MoveComponent`))
    ;[1 0.9983 0] HUD Visibility
    (set `self.HUDVisible` true)
    (else
      (set `self.HUDVisible` false)
      (goto _label_4 :!via `Reset`))))

(event `On Landed`
  (bind (_returnvalue_x _returnvalue_y _returnvalue_z) (`KismetMathLibrary.BreakVector` (`SceneComponent.K2_GetComponentLocation` (`self.Box`))))
  (bind (_returnvalue_x_2 _returnvalue_y_2 _returnvalue_z_2) (`KismetMathLibrary.BreakVector` (`SceneComponent.K2_GetComponentLocation` (`self.Box`))))
  (bind (_outhit _returnvalue) (`KismetSystemLibrary.LineTraceSingle` (`KismetMathLibrary.MakeVector` _returnvalue_x _returnvalue_y (- _returnvalue_z 30.0)) (- (`KismetMathLibrary.MakeVector` _returnvalue_x_2 _returnvalue_y_2 (- _returnvalue_z_2 30.0)) (0.0 0.0 10.0)) "TraceTypeQuery1"))
  (if _returnvalue
    (if (and _returnvalue (`self.NotLanded`))
      (`|ExecutionSequence`
        (:`then_1`
          (set `self.NotLanded` false)
          (`KismetSystemLibrary.PrintString` "")
          (set `/Game/Blueprints/BP_MoveComponent.DragMultiplier` (`KismetMathLibrary.FClamp` (+ (`/Game/Blueprints/BP_MoveComponent.DragMultiplier` (`self.BP_MoveComponent`)) 0.2) 0.0 0.9) (`self.BP_MoveComponent`))
          (set `self.EnergyCounter` 0)
          (set `self.Energy Depleted` false)
          (`PaperFlipbookComponent.SetFlipbook` (`self.SpriteFB`) "/Game/Assets/2D/2d_character_asset/animations/FP_landing.FP_landing")
          (`KismetSystemLibrary.RetriggerableDelay` 0.15)
          (`PaperFlipbookComponent.SetFlipbook` (`self.SpriteFB`) "/Game/Assets/2D/2d_character_asset/animations/FP_Idle.FP_Idle")
          ;[1 0.07208 0] On Landed Anim
          (`self.landsquash`))))
    (else
      (set `self.NotLanded` true)
      (if (< (`self.EnergyCounter`) 1)
        (set `self.EnergyCounter` 1)))))

(event `CustomEvent`)

(event `self.Box.OnComponentBeginOverlap`
  (params (OverlappedComponent :type "PrimitiveComponent Object Reference") (OtherActor :type "Actor Object Reference") (OtherComp :type "PrimitiveComponent Object Reference") (OtherBodyIndex :type Integer) (bFromSweep :type Boolean) (SweepResult :type "HitResult Structure (by ref)"))
  (bind _returnvalue (`GameplayStatics.GetPlayerController` 0))
  (cast `/Game/Blueprints/BP_EndZone` OtherActor)
  (set `PlayerController.bShowMouseCursor` true _returnvalue)
  (bind _returnvalue_2 (`|CreateWidget` "/Game/Blueprints/WPB_EndScreen.WPB_EndScreen_C" _returnvalue))
  (`UserWidget.AddToViewport` _returnvalue_2 0)
  (`WidgetBlueprintLibrary.SetInputMode_UIOnlyEx` (`GameplayStatics.GetPlayerController` 0) null)
  (`self.ConsumeMovementInputVector`)
  (set `self.Movement Input Check` false))

(fn `Dash Function`
  (params (`Direction Multiplier` :type "Float (double-precision)"))
  (locals (VelocityBeforeDash :type "Float (double-precision)"))
  (bind _bp_movecomponent (`self.BP_MoveComponent`))
  (bind (_returnvalue_x _returnvalue_y _returnvalue_z) (`KismetMathLibrary.BreakVector` (* (`/Game/Blueprints/BP_MoveComponent.Velocity` _bp_movecomponent) -1.0)))
  (`/Game/Blueprints/BP_MoveComponent.Deconfigure Physics` _bp_movecomponent)
  (set `self.Movement Input Check` false)
  (`PrimitiveComponent.AddImpulse` (`self.Box`) (`KismetMathLibrary.MakeVector` _returnvalue_x _returnvalue_y _returnvalue_z) "None" true)
  (`/Game/Blueprints/BP_MoveComponent.Configure Physics` (`self.BP_MoveComponent`))
  (set `self.Movement Input Check` true))

(fn `DashTrace`
  (bind (_returnvalue_x _returnvalue_y _returnvalue_z) (`KismetMathLibrary.BreakVector` (+ (`SceneComponent.GetRightVector` (`self.Box`)) (`SceneComponent.K2_GetComponentLocation` (`self.Box`)))))
  (if (`self.MovingRight`)
    (`KismetSystemLibrary.LineTraceSingle` :`Start` (`SceneComponent.K2_GetComponentLocation` (`self.Box`)) :`End` (`KismetMathLibrary.MakeVector` _returnvalue_x (+ _returnvalue_y 400.0) _returnvalue_z) :`TraceChannel` "TraceTypeQuery1" :`DrawDebugType` "ForDuration")))

(fn `Energy System`
  (returns (`Energy Remaining` :type Integer))
  (bind _aswbp_hud (cast `/Game/Blueprints/WBP_Hud` (`WidgetComponent.GetUserWidgetObject` (`self.HUD`))))
  (`/Game/Blueprints/WBP_Hud.EnergyResponse` _aswbp_hud)
  (bind _output_get (set `self.EnergyCounter` (+ (`self.EnergyCounter`) 1)))
  (if (>= _output_get (`self.Max Energy`))
    (set `self.Energy Depleted` true))
  (return _output_get))

(fn `Jump Function`
  (params (`Jump Strength Modifier` :type "Float (double-precision)") (`Jump Strength` :type "Float (double-precision)"))
  (bind (_velocity_x _velocity_y _velocity_z) (`KismetMathLibrary.BreakVector` (`/Game/Blueprints/BP_MoveComponent.Velocity` (`self.BP_MoveComponent`))))
  (bind _returnvalue (* _velocity_z -1.0))
  (`KismetSystemLibrary.PrintString` (`KismetStringLibrary.Conv_DoubleToString` _returnvalue))
  (`KismetSystemLibrary.PrintString` (`KismetStringLibrary.Conv_DoubleToString` _velocity_z))
  (`PrimitiveComponent.AddImpulse` (`self.Box`) (`KismetMathLibrary.MakeVector` 0.0 0.0 (+ `Jump Strength` _returnvalue)) "None" true))

(fn `UpdateHUD`
  (cast `/Game/Blueprints/WBP_Hud` (`WidgetComponent.GetUserWidgetObject` (`self.HUD`)))
  (return))

(fn `UserConstructionScript`)
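; BP_Blorb is a collectible that plays an idle flipbook and sound on spawn and is picked up when BP_Player overlaps it.
; Pickup increments the blorb's own BlorbsAcquired variable, switches to the consumed flipbook, disables Sphere1 collision and plays a splosion sound.
; After a short delay for the effect, it destroys the Pulse component and itself.
; PaperZD animation-instance nodes are present but never run.
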(event `self.ReceiveBeginPlay`
  (`PaperFlipbookComponent.SetFlipbook` (`self.FB_Blorb`) "/Game/Assets/2D/blorbflipbook/blorbspirtes/FP_idleblorb.FP_idleblorb")
  (`GameplayStatics.PlaySoundAtLocation` "/Game/Assets/sfx/blorbidlesfx_Cue.blorbidlesfx_Cue" (`self.K2_GetActorLocation`) (struct) 1.0 1.0 0.0 "/Game/Assets/sfx/blorbattenuation.blorbattenuation" null null null))

(event `self.ReceiveActorBeginOverlap`
  (params (OtherActor :type "Actor Object Reference"))
  (cast `/Game/Blueprints/BP_Player` OtherActor)
  (set `self.BlorbsAcquired` (+ 1.0 (`self.BlorbsAcquired`)))
  (`PaperFlipbookComponent.SetFlipbook` (`self.FB_Blorb`) "/Game/Assets/2D/blorbflipbook/blorbspirtes/FP_Blorbconsumed.FP_Blorbconsumed")
  (`PrimitiveComponent.SetCollisionEnabled` (`self.Sphere1`) "NoCollision")
  (`GameplayStatics.PlaySoundAtLocation` "/Game/Assets/sfx/blorbsplosionsfx.blorbsplosionsfx" (`self.K2_GetActorLocation`) (struct) 0.85 1.0 0.0 null null null null)
  (`KismetSystemLibrary.Delay` 0.66)
  (`ActorComponent.K2_DestroyComponent` (`self.pulse`))
  (`self.K2_DestroyActor`))

(fn `UserConstructionScript`)
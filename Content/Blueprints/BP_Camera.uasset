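; Side-scrolling camera actor that takes over the player's view and follows a target actor along Y and Z at a fixed world X.
; Construction script snaps it beside the target and yaws toward it.
; Each tick, dead-zone functions update the desired position, with optional fixed Z, height cap and Z offset.
; Movement lerps toward that position by a drag alpha, without delta-time scaling.
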(event `self.ReceiveBeginPlay`
  (`PlayerController.SetViewTargetWithBlend` (`GameplayStatics.GetPlayerController` 0) self 0.0 "VTBlend_Linear" 0.0 false))

(event `self.ReceiveTick`
  (params (DeltaSeconds :type "Float (single-precision)"))
  (bind (_returnvalue_x _returnvalue_y _returnvalue_z) (`KismetMathLibrary.BreakVector` (`self.K2_GetActorLocation`)))
  (bind _maxcameraheight (`self.MaxCameraHeight`))
  (bind _newy (`self.GetNewYValue`))
  (bind _output_get (set `self.CameraY` _newy))
  (bind _newz (`self.GetNewZValue`))
  (bind _output_get_2 (set `self.CameraZ` _newz))
  (if (and (> _output_get_2 _maxcameraheight) (!= _maxcameraheight 0.0))
    (set `self.CameraZ` (`self.MaxCameraHeight`)))
  (`self.K2_SetActorLocation` (`KismetMathLibrary.VLerp` (`KismetMathLibrary.MakeVector` _returnvalue_x _returnvalue_y _returnvalue_z) (`KismetMathLibrary.MakeVector` (`self.DistanceFromTarget`) _output_get (+ _output_get_2 (`self.ZOffset`))) (`self.CameraDrag`))))

(fn `GetNewYValue`
  (returns (NewY :type "Float (double-precision)"))
  (bind (_returnvalue_x _returnvalue_y) (`KismetMathLibrary.BreakVector` (`self.K2_GetActorLocation`)))
  (bind (_returnvalue_x_2 _returnvalue_y_2) (`KismetMathLibrary.BreakVector` (`self.K2_GetActorLocation`)))
  (bind (_returnvalue_x_3 _returnvalue_y_3) (`KismetMathLibrary.BreakVector` (`self.K2_GetActorLocation` (`self.ActorToFollow`))))
  (bind (_returnvalue_x_4 _returnvalue_y_4) (`KismetMathLibrary.BreakVector` (`self.K2_GetActorLocation` (`self.ActorToFollow`))))
  (bind _returnvalue (- _returnvalue_y_4 (`self.YDeadZone`)))
  (bind _returnvalue_2 (+ _returnvalue_y_3 (`self.YDeadZone`)))
  (if (> _returnvalue _returnvalue_y_2)
    (return _returnvalue)
    (elif (< _returnvalue_2 _returnvalue_y)
      (return _returnvalue_2)
      (else
        (return (`self.CameraY`))))))

(fn `GetNewZValue`
  (returns (NewZ :type "Float (double-precision)"))
  (bind (_returnvalue_x _returnvalue_y _returnvalue_z) (`KismetMathLibrary.BreakVector` (`self.K2_GetActorLocation`)))
  (bind (_returnvalue_x_2 _returnvalue_y_2 _returnvalue_z_2) (`KismetMathLibrary.BreakVector` (`self.K2_GetActorLocation`)))
  (bind (_returnvalue_x_3 _returnvalue_y_3 _returnvalue_z_3) (`KismetMathLibrary.BreakVector` (`self.K2_GetActorLocation` (`self.ActorToFollow`))))
  (bind (_returnvalue_x_4 _returnvalue_y_4 _returnvalue_z_4) (`KismetMathLibrary.BreakVector` (`self.K2_GetActorLocation` (`self.ActorToFollow`))))
  (bind _returnvalue (- _returnvalue_z_3 (`self.ZDeadZone`)))
  (bind _returnvalue_2 (+ _returnvalue_z_4 (`self.ZDeadZone`)))
  (if (!= (`self.FixedZValue`) 0.0)
    (return (`self.FixedZValue`))
    (elif (> _returnvalue (- _returnvalue_z (`self.ZOffset`)))
      (return _returnvalue)
      (elif (< _returnvalue_2 (- _returnvalue_z_2 (`self.ZOffset`)))
        (return _returnvalue_2)
        (else
          (return (`self.CameraZ`)))))))

(fn `UserConstructionScript`
  (bind _actortofollow (`self.ActorToFollow`))
  (bind (_returnvalue_x _returnvalue_y _returnvalue_z) (`KismetMathLibrary.BreakVector` (`self.K2_GetActorLocation` _actortofollow)))
  (bind (_returnvalue_roll _returnvalue_pitch _returnvalue_yaw) (`KismetMathLibrary.BreakRotator` (`KismetMathLibrary.FindLookAtRotation` (`self.K2_GetActorLocation`) (`self.K2_GetActorLocation` (`self.ActorToFollow`)))))
  (`/Engine/EditorBlueprintResources/StandardMacros.IsValid` _actortofollow
    (:`Is Valid`
      (bind _output_get (set `self.CameraY` _returnvalue_y))
      (if (!= (`self.FixedZValue`) 0.0)
        (set `self.CameraZ` (`self.FixedZValue`))
        (else
          (bind _output_get_2 (set `self.CameraZ` (+ _returnvalue_z (`self.ZDeadZone`))))))
      (`self.K2_SetActorLocation` (`KismetMathLibrary.MakeVector` (`self.DistanceFromTarget`) _output_get _output_get_2))
      (`self.K2_SetActorRotation` (`KismetMathLibrary.MakeRotator` 0.0 0.0 _returnvalue_yaw)))))
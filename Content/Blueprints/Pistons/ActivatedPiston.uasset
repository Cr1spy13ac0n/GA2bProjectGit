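; Piston that activates when BP_Player overlaps its box, shaking its head and then launching its platform upward.
; The RiseAndFall timeline jitters the head around its start position and fires an event that starts the Launch timeline.
; Launch steps the platform up to Height, then Tick slowly lowers it back to its origin.
; The overlap guard blocks activation only when Falling and Rising are both true.
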(event `self.ReceiveBeginPlay`
  (set `self.P_OriginalLocation` (`SceneComponent.RelativeLocation` (`self.plat`)))
  (set `self.H_OriginalLocation` (`SceneComponent.RelativeLocation` (`self.Head`))))

(event `ActivatePiston`
  (bind (_p_originallocation_x _p_originallocation_y _p_originallocation_z) (`KismetMathLibrary.BreakVector` (`self.P_OriginalLocation`)))
  (bind (_relativelocation_x _relativelocation_y _relativelocation_z) (`KismetMathLibrary.BreakVector` (`SceneComponent.RelativeLocation` (`self.plat`))))
  (set `self.Rising` true)
  (`Timeline|Rise and Fall` :!via `PlayFromStart`
    (:`Update`
      (`self.Shake`))
    (:`Launch`
      (`KismetSystemLibrary.DelayUntilNextTick`)
      (`Timeline|Launch` :!via `PlayFromStart` :!label _label
        (:`Update`
          (if (< _relativelocation_z (+ _p_originallocation_z (`self.Height`)))
            (`SceneComponent.K2_AddLocalOffset` (`self.plat`) (0.0 0.0 30.0) false false)
            (else
              (`|ExecutionSequence`
                (:`then_0`
                  (goto _label :!via `Stop`))
                (:`then_1`
                  (set `self.Falling` true)
                  (set `self.Rising` false))))))))))

(event `self.ReceiveTick`
  (params (DeltaSeconds :type "Float (single-precision)"))
  (bind (_p_originallocation_x _p_originallocation_y _p_originallocation_z) (`KismetMathLibrary.BreakVector` (`self.P_OriginalLocation`)))
  (bind (_relativelocation_x _relativelocation_y _relativelocation_z) (`KismetMathLibrary.BreakVector` (`SceneComponent.RelativeLocation` (`self.plat`))))
  (if (`self.Falling`)
    (if (< _relativelocation_z _p_originallocation_z)
      (set `self.Falling` false)
      (else
        (`SceneComponent.K2_AddLocalOffset` (`self.plat`) (0.0 0.0 -2.0) false false)))))

(event `self.Box.OnComponentBeginOverlap`
  (params (OverlappedComponent :type "PrimitiveComponent Object Reference") (OtherActor :type "Actor Object Reference") (OtherComp :type "PrimitiveComponent Object Reference") (OtherBodyIndex :type Integer) (bFromSweep :type Boolean) (SweepResult :type "HitResult Structure (by ref)"))
  (if (== (`GameplayStatics.GetObjectClass` OtherActor) "/Game/Blueprints/BP_Player.BP_Player_C")
    (if (not (and (`self.Falling`) (`self.Rising`)))
      (`self.ActivatePiston`))))

(fn `Shake`
  (bind _output_get (set `self.Offset` (`KismetMathLibrary.MakeVector` 0.0 (`KismetMathLibrary.RandomFloatInRange` -5.0 5.0) (`KismetMathLibrary.RandomFloatInRange` -2.0 2.0))))
  (`SceneComponent.K2_SetRelativeLocation` (`self.Head`) (+ _output_get (`self.H_OriginalLocation`)) false false))

(fn `UserConstructionScript`)
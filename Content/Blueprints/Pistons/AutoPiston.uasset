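; Self-cycling piston that shakes as a warning, shoots its platform up to a set Height, then sinks back and repeats.
; The RiseAndFall timeline jitters the Head around its start position, then its Launch event dips the Plat and starts the Launch timeline.
; Launch raises the Plat in fixed per-update steps; Tick then lowers it more slowly and restarts RiseAndFall, so speeds depend on frame rate.
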(event `self.ReceiveBeginPlay`
  (bind (_p_originallocation_x _p_originallocation_y _p_originallocation_z) (`KismetMathLibrary.BreakVector` (`self.P_OriginalLocation`)))
  (bind (_relativelocation_x _relativelocation_y _relativelocation_z) (`KismetMathLibrary.BreakVector` (`SceneComponent.RelativeLocation` (`self.plat`))))
  (set `self.P_OriginalLocation` (`SceneComponent.RelativeLocation` (`self.plat`)))
  (set `self.H_OriginalLocation` (`SceneComponent.RelativeLocation` (`self.Head`)))
  (`Timeline|Rise and Fall` :!via `PlayFromStart` :!label _label
    (:`Update`
      (`self.Shake`))
    (:`Launch`
      (`SceneComponent.K2_AddLocalOffset` (`self.plat`) (0.0 0.0 -5.0) false false)
      (`KismetSystemLibrary.DelayUntilNextTick`)
      (`Timeline|Launch` :!via `PlayFromStart` :!label _label_2
        (:`Update`
          (if (< _relativelocation_z (+ _p_originallocation_z (`self.Height`)))
            (`SceneComponent.K2_AddLocalOffset` (`self.plat`) (0.0 0.0 20.0) false false)
            (else
              (set `self.Falling` true)
              (goto _label_2 :!via `Stop`))))))))

(event `self.ReceiveTick`
  (params (DeltaSeconds :type "Float (single-precision)"))
  (bind (_p_originallocation_x _p_originallocation_y _p_originallocation_z) (`KismetMathLibrary.BreakVector` (`self.P_OriginalLocation`)))
  (bind (_relativelocation_x _relativelocation_y _relativelocation_z) (`KismetMathLibrary.BreakVector` (`SceneComponent.RelativeLocation` (`self.plat`))))
  (if (`self.Falling`)
    (if (< _relativelocation_z _p_originallocation_z)
      (set `self.Falling` false)
      (goto _label :!via `PlayFromStart`)
      (else
        (`SceneComponent.K2_AddLocalOffset` (`self.plat`) (0.0 0.0 -2.0) false false)))))

(fn `Shake`
  (bind _output_get (set `self.Offset` (`KismetMathLibrary.MakeVector` 0.0 (`KismetMathLibrary.RandomFloatInRange` -5.0 5.0) (`KismetMathLibrary.RandomFloatInRange` -2.0 2.0))))
  (`SceneComponent.K2_SetRelativeLocation` (`self.Head`) (+ _output_get (`self.H_OriginalLocation`)) false false))

(fn `UserConstructionScript`)